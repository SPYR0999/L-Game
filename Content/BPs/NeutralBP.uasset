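; NeutralBP is a grid-aligned actor whose static mesh shifts between two vertical positions, around 19 and -210.
; BeginPlay repositions the actor through SnapToGrid, whose listed offset-snapping math is marked unused.
; Lift nudges the mesh by a fraction of GridSize, with direction set by a boolean and mirrored near the lower position.
; Invert flips the mesh between both heights, using a tolerant comparison to detect its current state.
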(event EventBeginPlay
  (Transformation|SetActorLocation (Utilities|SnaptoGrid (Transformation|GetActorLocation)) false false))

(fn ConstructionScript)

(fn Lift
  (params (True :type Boolean))
  (bind _returnvalue (select True 2.5 -2.5))
  (bind _staticmesh (Variables|Default|GetStaticMesh))
  (bind _gridsize (Variables|Default|GetGridSize))
  (bind _returnvalue_2 (/ _gridsize _returnvalue))
  (bind _relativelocation (Variables|/Script/Engine.SceneComponent|GetRelativeLocation _staticmesh))
  (bind (_x _y _z) (Math|Vector|BreakVector _relativelocation))
  (Transformation|SetRelativeLocation (Variables|Default|GetStaticMesh) (Math|Vector|MakeVector _x _y (select (Math|Float|NearlyEqual(Float) _z -2.1e+02 62.0) (- _z _returnvalue_2) (+ _z _returnvalue_2))) false false)
  (return))

(fn Invert
  (bind _staticmesh (Variables|Default|GetStaticMesh))
  (bind _relativelocation (Variables|/Script/Engine.SceneComponent|GetRelativeLocation _staticmesh))
  (bind (_x _y _z) (Math|Vector|BreakVector _relativelocation))
  (Transformation|SetRelativeLocation _staticmesh (Math|Vector|MakeVector _x _y (select (Math|Float|NearlyEqual(Float) _z 19.0 62.0) -2.1e+02 19.0)) false false)
  (return))